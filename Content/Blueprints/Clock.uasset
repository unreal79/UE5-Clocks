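; Clock actor that displays the system's current time as six digits (hours, minutes, seconds) on its mesh.
; The construction script creates a dynamic instance of the ClockDigit material for each digit's material slot on the Clock mesh.
; Every Tick reads Now(), splits each value into tens and units by repeated subtraction of ten, and sets each instance's Digit texture from the DigiNums array.
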(event EventBeginPlay)

(event Collision|EventActorBeginOverlap
  (params (OtherActor :type Actor%20Object%20Reference)))

(event EventTick
  (params (DeltaSeconds :type Float%20%28single-precision%29))
  (CallFunction|SetCurrentTime)
  (CallFunction|SetUpSingleDigits)
  (CallFunction|SetTextures))

(fn ConstructionScript
  (bind _returnvalue (Rendering|Material|CreateDynamicMaterialInstance "/Game/Materials/ClockDigit.ClockDigit" :!class /Script/Engine.KismetMaterialLibrary))
  (bind _output_get (Variables|Default|SetSecond_Dec _returnvalue))
  (Rendering|Material|SetMaterial (Variables|Default|GetClock) 1 _output_get)
  (bind _returnvalue_2 (Rendering|Material|CreateDynamicMaterialInstance "/Game/Materials/ClockDigit.ClockDigit" :!class /Script/Engine.KismetMaterialLibrary))
  (bind _output_get_2 (Variables|Default|SetSecond _returnvalue_2))
  (Rendering|Material|SetMaterial (Variables|Default|GetClock) 2 _output_get_2)
  (bind _returnvalue_3 (Rendering|Material|CreateDynamicMaterialInstance "/Game/Materials/ClockDigit.ClockDigit" :!class /Script/Engine.KismetMaterialLibrary))
  (bind _output_get_3 (Variables|Default|SetMinute_Dec _returnvalue_3))
  (Rendering|Material|SetMaterial (Variables|Default|GetClock) 3 _output_get_3)
  (bind _returnvalue_4 (Rendering|Material|CreateDynamicMaterialInstance "/Game/Materials/ClockDigit.ClockDigit" :!class /Script/Engine.KismetMaterialLibrary))
  (bind _output_get_4 (Variables|Default|SetMinute _returnvalue_4))
  (Rendering|Material|SetMaterial (Variables|Default|GetClock) 4 _output_get_4)
  (bind _returnvalue_5 (Rendering|Material|CreateDynamicMaterialInstance "/Game/Materials/ClockDigit.ClockDigit" :!class /Script/Engine.KismetMaterialLibrary))
  (bind _output_get_5 (Variables|Default|SetHour_Dec _returnvalue_5))
  (Rendering|Material|SetMaterial (Variables|Default|GetClock) 5 _output_get_5)
  (bind _returnvalue_6 (Rendering|Material|CreateDynamicMaterialInstance "/Game/Materials/ClockDigit.ClockDigit" :!class /Script/Engine.KismetMaterialLibrary))
  (bind _output_get_6 (Variables|Default|SetHour _returnvalue_6))
  (Rendering|Material|SetMaterial (Variables|Default|GetClock) 6 _output_get_6))

(fn SetCurrentTime
  (bind _returnvalue (Math|DateTime|Now))
  (bind (_year _month _day _hour _minute _second) (Math|DateTime|BreakDateTime _returnvalue))
  (Variables|Default|SetCurrentSecond _second)
  (Variables|Default|SetCurrentDecSecond 0)
  (Variables|Default|SetCurrentMinute _minute)
  (Variables|Default|SetCurrentDecMinute 0)
  (Variables|Default|SetCurrentHour _hour)
  (Variables|Default|SetCurrentDecHour 0))

(fn SetUpSingleDigits
  (if (>= (Variables|Default|GetCurrentSecond) 10) :!label _label
    (Variables|Default|SetCurrentDecSecond (+ (Variables|Default|GetCurrentDecSecond) 1))
    (Variables|Default|SetCurrentSecond (- (Variables|Default|GetCurrentSecond) 10))
    (goto _label)
    (else
      (if (>= (Variables|Default|GetCurrentMinute) 10) :!label _label_2
        (Variables|Default|SetCurrentDecMinute (+ (Variables|Default|GetCurrentDecMinute) 1))
        (Variables|Default|SetCurrentMinute (- (Variables|Default|GetCurrentMinute) 10))
        (goto _label_2)
        (else
          (if (>= (Variables|Default|GetCurrentHour) 10) :!label _label_3
            (Variables|Default|SetCurrentDecHour (+ (Variables|Default|GetCurrentDecHour) 1))
            (Variables|Default|SetCurrentHour (- (Variables|Default|GetCurrentHour) 10))
            (goto _label_3)))))))

(fn SetTextures
  (Rendering|Material|SetTextureParameterValue (Variables|Default|GetSecond_Dec) "Digit" (Utilities|Array|Get(acopy) (Variables|Default|GetDigiNums) (Variables|Default|GetCurrentDecSecond)))
  (Rendering|Material|SetTextureParameterValue (Variables|Default|GetSecond) "Digit" (Utilities|Array|Get(acopy) (Variables|Default|GetDigiNums) (Variables|Default|GetCurrentSecond)))
  (Rendering|Material|SetTextureParameterValue (Variables|Default|GetMinute_Dec) "Digit" (Utilities|Array|Get(acopy) (Variables|Default|GetDigiNums) (Variables|Default|GetCurrentDecMinute)))
  (Rendering|Material|SetTextureParameterValue (Variables|Default|GetMinute) "Digit" (Utilities|Array|Get(acopy) (Variables|Default|GetDigiNums) (Variables|Default|GetCurrentMinute)))
  (Rendering|Material|SetTextureParameterValue (Variables|Default|GetHour_Dec) "Digit" (Utilities|Array|Get(acopy) (Variables|Default|GetDigiNums) (Variables|Default|GetCurrentDecHour)))
  (Rendering|Material|SetTextureParameterValue (Variables|Default|GetHour) "Digit" (Utilities|Array|Get(acopy) (Variables|Default|GetDigiNums) (Variables|Default|GetCurrentHour))))