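; Analogue clock actor that rotates hour, minute and second hand meshes to show either real system time or a configurable start time plus accumulated elapsed seconds.
; BeginPlay starts an endless Delay loop that converts the time into negative relative pitch angles, with fractional offsets for gradual movement.
; SmoothSeconds selects rapid updates, otherwise the loop runs once per second and plays an attenuated tick sound at the face.
; Tick accumulates the elapsed seconds.
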(event EventBeginPlay
  (Variables|RealTime|SetStart%20Time (Math|DateTime|MakeDateTime 1 1 1 (Variables|RealTime|GetStart%20Time%20Hour) (Variables|RealTime|GetStart%20Time%20Minute) (Variables|RealTime|GetStart%20Time%20Second) 0))
  (if (Variables|Default|GetSmoothSeconds)
    (Variables|Default|SetDelay 0.02)
    (else
      (Variables|Default|SetDelay 1.0)))
  (Transformation|SetRelativeRotation (Variables|Default|GetHour%20Mesh) (Math|Rotator|MakeRotator 0.0 (- 0.0 (+ (Math|Conversions|ToFloat(Integer) (* (.Hour (Math|DateTime|BreakDateTime (select (Variables|RealTime|GetReal%20Time?) (Math|DateTime|Now) (+ (Variables|RealTime|GetStart%20Time) (Math|Timespan|FromSeconds (Variables|RealTime|GetDelta%20Seconds)))))) 30)) (/ (Math|Conversions|ToFloat(Integer) (.Minute (Math|DateTime|BreakDateTime (select (Variables|RealTime|GetReal%20Time?) (Math|DateTime|Now) (+ (Variables|RealTime|GetStart%20Time) (Math|Timespan|FromSeconds (Variables|RealTime|GetDelta%20Seconds))))))) 2.0))) 0.0) false false :!label _label)
  (Transformation|SetRelativeRotation (Variables|Default|GetMinute%20Mesh) (Math|Rotator|MakeRotator 0.0 (- 0.0 (+ (* (Math|Conversions|ToFloat(Integer) (.Minute (Math|DateTime|BreakDateTime (select (Variables|RealTime|GetReal%20Time?) (Math|DateTime|Now) (+ (Variables|RealTime|GetStart%20Time) (Math|Timespan|FromSeconds (Variables|RealTime|GetDelta%20Seconds))))))) 6.0) (/ (Math|Conversions|ToFloat(Integer) (.Second (Math|DateTime|BreakDateTime (select (Variables|RealTime|GetReal%20Time?) (Math|DateTime|Now) (+ (Variables|RealTime|GetStart%20Time) (Math|Timespan|FromSeconds (Variables|RealTime|GetDelta%20Seconds))))))) 1e+01))) 0.0) false false)
  (Transformation|SetRelativeRotation (Variables|Default|GetSecond%20Mesh) (Math|Rotator|MakeRotator 0.0 (- 0.0 (+ (* (Math|Conversions|ToFloat(Integer) (.Second (Math|DateTime|BreakDateTime (select (Variables|RealTime|GetReal%20Time?) (Math|DateTime|Now) (+ (Variables|RealTime|GetStart%20Time) (Math|Timespan|FromSeconds (Variables|RealTime|GetDelta%20Seconds))))))) 6.0) (* (/ (Math|Conversions|ToFloat(Integer) (.Millisecond (Math|DateTime|BreakDateTime (select (Variables|RealTime|GetReal%20Time?) (Math|DateTime|Now) (+ (Variables|RealTime|GetStart%20Time) (Math|Timespan|FromSeconds (Variables|RealTime|GetDelta%20Seconds))))))) 1e+03) 6.0))) 0.0) false false)
  (Utilities|FlowControl|Delay (Variables|Default|GetDelay))
  (if (Variables|Default|GetSmoothSeconds)
    (goto _label)
    (else
      (Audio|SpawnSoundatLocation (Variables|Sound|GetTick%20Sound) (Transformation|GetWorldLocation (Variables|Default|GetFace%20Mesh)) "0, 0, 0" (Variables|Sound|GetVolume%20Multiplier) 1.0 0.0 (Variables|Sound|GetAttenuation%20Settings) 0)
      (goto _label))))

(event EventTick
  (params (DeltaSeconds :type Float%20%28single-precision%29))
  (Variables|RealTime|SetDelta%20Seconds (+ DeltaSeconds (Variables|RealTime|GetDelta%20Seconds))))

(fn ConstructionScript)